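; BP_Projectile is a projectile that flies along world X and awards the player score when it hits an enemy.
; Tick moves it by ForwardSpeed, delta time and a Counter that grows every frame, so it accelerates at a frame-rate-dependent rate.
; Sphere overlaps ignore BP_Player, call IncreaseScore on the player pawn for BP_Enemy, then destroy the projectile.
; Any other overlap simply destroys the projectile.
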(event `self.ReceiveTick`
  (params (DeltaSeconds :type "Float (single-precision)"))
  (bind _output_get (set `self.Counter` (+ (`self.Counter`) 0.0003)))
  (`self.K2_AddActorWorldOffset` (`KismetMathLibrary.MakeVector` (* DeltaSeconds (`self.ForwardSpeed`) _output_get))))

(event `self.Sphere.OnComponentBeginOverlap`
  (params (OverlappedComponent :type "PrimitiveComponent Object Reference") (OtherActor :type "Actor Object Reference") (OtherComp :type "PrimitiveComponent Object Reference") (OtherBodyIndex :type Integer) (bFromSweep :type Boolean) (SweepResult :type "HitResult Structure (by ref)"))
  (cast `/Game/InfiniteMatrix/Blueprints/BP_Player` OtherActor
    (:`CastFailed`
      (cast `/Game/InfiniteMatrix/Blueprints/BP_Enemy` OtherActor
        (:`then`
          (bind _asbp_player (cast `/Game/InfiniteMatrix/Blueprints/BP_Player` (`GameplayStatics.GetPlayerPawn` 0)))
          (`/Game/InfiniteMatrix/Blueprints/BP_Player.IncreaseScore` _asbp_player)
          (`self.K2_DestroyActor`))
        (:`CastFailed`
          (`self.K2_DestroyActor`))))))

(fn `UserConstructionScript`)